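; AnchorsConfig is a configuration Blueprint that starts anchor placement when play begins.
; On BeginPlay it spawns an AnchorPlacer at the world origin, passing in its match threshold, interior and exterior anchor classes, alignment parent and IP address.
; Outside the preparation stage, it also calls AddChangeMode on the Player.
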(event `self.ReceiveBeginPlay`
  (`|SpawnActorFromClass` "/LASAA/Blueprints/AnchorPlacer.AnchorPlacer_C" (`KismetMathLibrary.MakeTransform` (0.0 0.0 0.0)) "Undefined" "MultiplyWithRoot" null (`self.MinNumberMatches`) (`self.INTAnchorClass`) (`self.EXTAnchorClass`) (`self.AnchorParent`) (`self.IPAddress`) null)
  (if (not (`self.Preparation stage`))
    (`AddComponent|NODE_AddChangeMode-1` :`self` (`self.Player`))))

(fn `UserConstructionScript`)