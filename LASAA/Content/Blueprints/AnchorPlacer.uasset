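; Places, saves, reloads and resets paired internal/external anchors that feed an alignment component, coordinated over OSC with ALVR and an external camera tracker.
; Input actions send place/reset commands; BeginPlay requests saved anchors by UUID, and replies spawn, move or reset them.
; A placed-anchor reply waits for a well-matched camera pose, converted from OpenCV to Unreal space.
; External anchors attach to the alignment parent, and internal anchors store the pairing and calibration offset.
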(event `EnhancedInput|/LASAA/InputActions/IA_ResetAnchors`
  (params (ActionValue :type Boolean) (ElapsedSeconds :type "Float (double-precision)") (TriggeredSeconds :type "Float (double-precision)") (InputAction :type "InputAction Object Reference" :default "/LASAA/InputActions/IA_ResetAnchors.IA_ResetAnchors"))
  ;[1 1 1] Anchor input message
  ;;[1 1 1] Reset all anchors
  (:`Triggered`
    (`self.Send Osc Command` (stale `self.ReceiveBeginPlay` _returnvalue_3) "/reset_anchors" (make `OSCMessage`))))

(event `EnhancedInput|/LASAA/InputActions/IA_PlaceAnchor`
  (params (ActionValue :type Boolean) (ElapsedSeconds :type "Float (double-precision)") (TriggeredSeconds :type "Float (double-precision)") (InputAction :type "InputAction Object Reference" :default "/LASAA/InputActions/IA_PlaceAnchor.IA_PlaceAnchor"))
  ;[1 1 1] Anchor input message
  ;;[1 1 1] Place a new anchor
  (:`Triggered`
    (`self.Send Osc Command` (stale `self.ReceiveBeginPlay` _returnvalue_3) "/place_anchor" (make `OSCMessage`))))

(event `self.ReceiveBeginPlay`
  ;[1 1 1] Setup
  (bind _returnvalue (`OSCManager.CreateOSCServer` "" 8001 false true "" self))
  (add `OSCServer.OnOscMessageReceived` _returnvalue (delegate `OnExtRecieved`))
  (bind _returnvalue_2 (`OSCManager.CreateOSCServer` "" 8002 false true "" self))
  (add `OSCServer.OnOscMessageReceived` _returnvalue_2 (delegate `CustomEvent`))
  (bind _returnvalue_3 (`OSCManager.CreateOSCClient` (`self.IPAddress`) 8002 "" self))
  (`AddComponent|NODE_AddAlignmentComponent-2` :`self` (`self.AllignmentParent`) :`m_extAnchorClass` (`self.EXTAnchorClass`) :`m_intAnchorClass` (`self.INTAnchorClass`))
  ;[1 1 1] Anchor input message
  ;;[1 1 1] Load all anchors
  (bind _uuids (`Anchor.loadAnchors`))
  (for _array_element _uuids
    (bind _returnvalue_4 (`OSCManager.AddString` (make `OSCMessage`) _array_element)))
  (`self.Send Osc Command` _returnvalue_3 "/load_anchors" _returnvalue_4))

(event `CustomEvent`
  (params (Message :type "OSCMessage Structure (by ref)") (IPAddress :type String) (Port :type Integer))
  ;[1 1 1] Anchor output messages
  (if (`KismetStringLibrary.EqualEqual_StrStr` IPAddress (`self.IPAddress`))
    (bind _oscmessageoutput (`self.IsAddressEqual` Message "/anchor_locations")
      (:`Equal`
        (bind _values (`OSCManager.GetAllFloats` _oscmessageoutput))
        (bind _values_2 (`OSCManager.GetAllStrings` _oscmessageoutput))
        (bind (_uuids _transforms) (`Anchor.TransformOSCALVRMessage` _values _values_2))
        (bind _outactors (`GameplayStatics.GetAllActorsOfClass` "/LASAA/Blueprints/Anchor_BP.Anchor_BP_C"))
        (for _array_element _outactors
          (bind _returnvalue (`Anchor.getUuid` _array_element))
          (`self.K2_SetActorTransform` _array_element (`|GetArrayItem` _transforms (`KismetArrayLibrary.Array_Find` _uuids _returnvalue)) false false)))
      (:`NotEqual`
        (`self.IsAddressEqual` Message "/anchors_reset"
          (:`Equal`
            (`Anchor.resetAnchors`))
          (:`NotEqual`
            (bind _oscmessageoutput_2 (`self.IsAddressEqual` Message "/anchors_loaded")
              (:`Equal`
                (bind _values_3 (`OSCManager.GetAllFloats` _oscmessageoutput_2))
                (bind _values_4 (`OSCManager.GetAllStrings` _oscmessageoutput_2))
                (bind (_uuids_2 _transforms_2) (`Anchor.TransformOSCALVRMessage` _values_3 _values_4))
                (bind (_uuids_3 _transforms_3) (`Anchor.loadAnchors`))
                (for (_array_element_2 _array_index) _uuids_2
                  (`self.SpawnAnchors` _array_element_2 (`self.AllignmentParent`) (`|GetArrayItem` _transforms_2 _array_index) (`|GetArrayItem` _transforms_3 (`KismetArrayLibrary.Array_Find` _uuids_3 _array_element_2)))))
              (:`NotEqual`
                (bind _oscmessageoutput_3 (`self.IsAddressEqual` Message "/anchor_placed")
                  (:`Equal`
                    (bind _values_5 (`OSCManager.GetAllFloats` _oscmessageoutput_3))
                    (bind _values_6 (`OSCManager.GetAllStrings` _oscmessageoutput_3))
                    (bind (_uuids_4 _transforms_4) (`Anchor.TransformOSCALVRMessage` _values_5 _values_6))
                    (set `self.PlaceAnchor` true)))))))))))

(event `OnExtRecieved`
  (params (Message :type "OSCMessage Structure (by ref)") (IPAddress :type String) (Port :type Integer))
  ;[1 1 1] On OSC External Camera Received
  ;;[1 1 1] Only continue when an anchor needs to be placed, and if tracking state is 0
  (bind _value (`OSCManager.GetInt32` Message))
  (if (== _value 0)
    (bind _transform (`self.TransformOSCExternalPackage` Message))
    ;;[1 1 1] Make sure enough matches were found
    (`OSCManager.GetInt32` Message 17) ; KFid
    (bind _value_2 (`OSCManager.GetInt32` Message 18)) ; nrMatches
    (if (> _value_2 (`self.MinNumberMatches`))
      (if (== (`self.PlaceAnchor`) true)
        ;;[1 1 1] Place both INT and EXT anchors
        (set `self.PlaceAnchor` false)
        (bind (_extanchor _intanchor) (`self.SpawnAnchors` (`|GetArrayItem` (stale `CustomEvent` _uuids_4)) (`self.AllignmentParent`) (`|GetArrayItem` (stale `CustomEvent` _transforms_4)) _transform))
        (`Anchor.saveAnchor` _intanchor)
        (`KismetSystemLibrary.PrintText` "ANCHORPLACED")))))

(fn `Send Osc Command`
  (params (OscClient :type "OSCClient Object Reference") (address :type String) (message :type "OSCMessage Structure"))
  (bind _returnvalue (`OSCManager.ConvertStringToOSCAddress` address))
  (bind _returnvalue_2 (`OSCManager.SetOSCMessageAddress` message _returnvalue))
  (`OSCClient.SendOSCMessage` OscClient _returnvalue_2)
  (return))

(fn `TransformOSCExternalPackage`
  (params (Message :type "OSCMessage Structure (by ref)"))
  (returns (Transform :type "Transform Structure"))
  (bind _value (`OSCManager.GetFloat` Message 1))
  (bind _value_2 (`OSCManager.GetFloat` Message 2))
  (bind _value_3 (`OSCManager.GetFloat` Message 3))
  (bind _value_4 (`OSCManager.GetFloat` Message 4))
  (bind _value_5 (`OSCManager.GetFloat` Message 5))
  (bind _value_6 (`OSCManager.GetFloat` Message 6))
  (bind _value_7 (`OSCManager.GetFloat` Message 7))
  (bind _value_8 (`OSCManager.GetFloat` Message 8))
  (bind _value_9 (`OSCManager.GetFloat` Message 9))
  (bind _value_10 (`OSCManager.GetFloat` Message 10))
  (bind _value_11 (`OSCManager.GetFloat` Message 11))
  (bind _value_12 (`OSCManager.GetFloat` Message 12))
  (bind _value_13 (`OSCManager.GetFloat` Message 13))
  (bind _value_14 (`OSCManager.GetFloat` Message 14))
  (bind _value_15 (`OSCManager.GetFloat` Message 15))
  (bind _value_16 (`OSCManager.GetFloat` Message 16))
  (bind _returnvalue (`Helper.ConvertOpenCVToUnreal` (`KismetMathLibrary.Conv_MatrixToTransform` (`KismetMathLibrary.Matrix_GetTransposed` (make `Matrix` (make `Plane` (* 100.0 _value_4) _value _value_2 _value_3) (make `Plane` (* 100.0 _value_8) _value_5 _value_6 _value_7) (make `Plane` (* 100.0 _value_12) _value_9 _value_10 _value_11) (make `Plane` _value_16 _value_13 _value_14 _value_15))))))
  (return _returnvalue))

(fn `UserConstructionScript`)